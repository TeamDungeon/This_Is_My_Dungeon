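; BP_Trap_Spike is a spike trap that damages a Hero entering its Radius overlap.
; On overlap it plays the SpikeTrap_HideAnimation_Anim animation once and calls GetDamaged if CanDamage is set.
; A one-second timer, started on each overlap, restores CanDamage as a hit cooldown.
; End overlap updates IsActive and, after a delay, CanHide, though nothing here reads either flag.
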(event OnComponentBeginOverlap(Radius)
  (params (OverlappedComponent :type Primitive%20Component%20Object%20Reference) (OtherActor :type Actor%20Object%20Reference) (OtherComp :type Primitive%20Component%20Object%20Reference) (OtherBodyIndex :type Integer) (bFromSweep :type Boolean) (SweepResult :type Hit%20Result%20Structure%20%28by%20ref%29))
  (bind _ashero (Utilities|Casting|CastToHero OtherActor))
  (Components|Animation|PlayAnimation (Variables|Default|GetSkeletalMesh) "/Game/Blueprints/Traps/SpikeTrap/Content/SpikeTrap_HideAnimation_Anim.SpikeTrap_HideAnimation_Anim" false)
  (CallFunction|CanDamageTimer)
  (if (Variables|Default|GetCanDamage)
    (Variables|Default|SetCanDamage false)
    (Class|MyEntity|GetDamaged _ashero (Variables|Default|GetDamage))))

(event OnComponentEndOverlap(Radius)
  (params (OverlappedComponent :type Primitive%20Component%20Object%20Reference) (OtherActor :type Actor%20Object%20Reference) (OtherComp :type Primitive%20Component%20Object%20Reference) (OtherBodyIndex :type Integer))
  (Utilities|Casting|CastToHero OtherActor)
  (Variables|Default|SetIsActive false)
  (Utilities|FlowControl|Delay 0.65)
  (Variables|Default|SetCanHide true))

(event Custom|CanDamageTimer
  (bind _returnvalue (Utilities|Time|SetTimerbyEvent (delegate Custom|ResetCanDamage) 1.0)))

(event Custom|ResetCanDamage
  (Variables|Default|SetCanDamage true)
  (Utilities|Time|ClearandInvalidateTimerbyHandle (stale Custom|CanDamageTimer _returnvalue)))

(fn ConstructionScript)