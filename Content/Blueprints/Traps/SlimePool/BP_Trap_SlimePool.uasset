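; BP_Trap_SlimePool is a slime pool trap that slows heroes standing inside its Radius volume.
; On overlap begin, a hero is added to TargetQueue and its max walk speed is set from its Speed scaled by SpeedMultiplier.
; On overlap end, the queued hero's ResetSpeedTimer is called with SlownessDuration, without removing it from the queue.
; Both events compare first child components to filter overlaps to the hero's capsule.
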(event OnComponentBeginOverlap(Radius)
  (params (OverlappedComponent :type Primitive%20Component%20Object%20Reference) (OtherActor :type Actor%20Object%20Reference) (OtherComp :type Primitive%20Component%20Object%20Reference) (OtherBodyIndex :type Integer) (bFromSweep :type Boolean) (SweepResult :type Hit%20Result%20Structure%20%28by%20ref%29))
  (bind _asbp_hero_base (Utilities|Casting|CastToBP_Hero_BASE OtherActor))
  (if (== (Components|GetChildComponent (Variables|/Script/Engine.Character|GetCapsuleComponent _asbp_hero_base) 0) (Components|GetChildComponent OtherComp 0))
    (Utilities|Array|Add (Variables|Default|GetTargetQueue) _asbp_hero_base)
    (Variables|/Script/Engine.CharacterMovementComponent|SetMaxWalkSpeed (Variables|/Script/Engine.Character|GetCharacterMovement _asbp_hero_base) (* (* (Variables|/Script/ThisIsMyDungeon.MyEntity|Getspeed _asbp_hero_base) (Variables|Default|GetSpeedMultiplier)) 1e+02))))

(event OnComponentEndOverlap(Radius)
  (params (OverlappedComponent :type Primitive%20Component%20Object%20Reference) (OtherActor :type Actor%20Object%20Reference) (OtherComp :type Primitive%20Component%20Object%20Reference) (OtherBodyIndex :type Integer))
  (bind _targetqueue (Variables|Default|GetTargetQueue))
  (bind _asbp_hero_base (Utilities|Casting|CastToBP_Hero_BASE OtherActor))
  (if (== (Components|GetChildComponent (Variables|/Script/Engine.Character|GetCapsuleComponent _asbp_hero_base) 0) (Components|GetChildComponent OtherComp 0))
    (Default|ResetSpeedTimer (Utilities|Array|Get(acopy) _targetqueue (Utilities|Array|FindItem _targetqueue _asbp_hero_base)) (Variables|Default|GetSlownessDuration))))

(fn ConstructionScript)