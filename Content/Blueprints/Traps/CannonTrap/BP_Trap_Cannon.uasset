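; BP_Trap_Cannon is a trap that turns toward heroes within its radius and fires cannonballs at them.
; Radius overlaps add and remove BP_Hero_BASE actors in a queue, filtered by a capsule child-component comparison.
; Each tick it yaws toward the first queued hero and attempts a shot, launching BP_CannonBall from the Nose socket with a forward impulse.
; A CanShoot flag gates firing until a ShootSpeed timer resets it and clears itself.
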(event OnComponentBeginOverlap(Radius)
  (params (OverlappedComponent :type Primitive%20Component%20Object%20Reference) (OtherActor :type Actor%20Object%20Reference) (OtherComp :type Primitive%20Component%20Object%20Reference) (OtherBodyIndex :type Integer) (bFromSweep :type Boolean) (SweepResult :type Hit%20Result%20Structure%20%28by%20ref%29))
  ;[1 1 1] In Radius
  (bind _asbp_hero_base (Utilities|Casting|CastToBP_Hero_BASE OtherActor))
  (if (== (Components|GetChildComponent (Variables|/Script/Engine.Character|GetCapsuleComponent _asbp_hero_base) 0) (Components|GetChildComponent OtherComp 0))
    (Utilities|Array|Add (Variables|Default|GetTargetQueue) _asbp_hero_base)))

(event OnComponentEndOverlap(Radius)
  (params (OverlappedComponent :type Primitive%20Component%20Object%20Reference) (OtherActor :type Actor%20Object%20Reference) (OtherComp :type Primitive%20Component%20Object%20Reference) (OtherBodyIndex :type Integer))
  ;[1 1 1] Out of Radius
  (bind _asbp_hero_base (Utilities|Casting|CastToBP_Hero_BASE OtherActor))
  (if (== (Components|GetChildComponent (Variables|/Script/Engine.Character|GetCapsuleComponent _asbp_hero_base) 0) (Components|GetChildComponent OtherComp 0))
    (Utilities|Array|RemoveItem (Variables|Default|GetTargetQueue) _asbp_hero_base)))

(event Custom|ShootTimer
  ;[1 1 1] Shoot timer
  (bind _returnvalue (Utilities|Time|SetTimerbyEvent (delegate Custom|ResetShoot) (Variables|Default|GetShootSpeed) true)))

(event Custom|ResetShoot
  ;[1 1 1] Shoot timer
  (Variables|Default|SetCanShoot true)
  (Utilities|Time|ClearandInvalidateTimerbyHandle (stale Custom|ShootTimer _returnvalue)))

(event Custom|Shoot
  ;[1 1 1] Shoot BP Cannon Ball
  (if (Variables|Default|GetCanShoot)
    (Variables|Default|SetCanShoot false)
    (bind _returnvalue (Game|SpawnActorfromClass "/Game/Blueprints/Traps/CannonTrap/BP_CannonBall.BP_CannonBall_C" (Math|Transform|MakeTransform (Transformation|GetSocketLocation (Variables|Default|GetStaticMesh) "Nose") "0, 0, 0" "1.000000,1.000000,1.000000") "Undefined" "MultiplyWithRoot" 0 0))
    (Class|PrimitiveComponent|AddVelocityChangeImpulseatLocation (Variables|/Game/Blueprints/Traps/CannonTrap/BP_CannonBall.BP_CannonBall_C|GetSphere _returnvalue) (* (Transformation|GetActorForwardVector) "10000.000000,10000.000000,10000.000000") "0, 0, 0" "None")
    (CallFunction|ShootTimer)))

(event EventTick
  (params (DeltaSeconds :type Float%20%28single-precision%29))
  ;[1 1 1] Update Rotation
  (if (Utilities|Array|IsNotEmpty (Variables|Default|GetTargetQueue))
    (Transformation|SetActorRotation (Math|Rotator|MakeRotator 0.0 0.0 (.yaw (Math|Rotator|FindLookatRotation (Transformation|GetActorLocation) (Transformation|GetActorLocation (Utilities|Array|Get(acopy) (Variables|Default|GetTargetQueue)))))))
    (CallFunction|Shoot)))

(fn ConstructionScript)