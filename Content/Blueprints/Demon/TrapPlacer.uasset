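; TrapPlacer is a controllable pawn that acts as a cursor for placing traps in an edit mode.
; On BeginPlay it adds its Enhanced Input mapping context to the player controller's input subsystem.
; The move action feeds movement input along world X and Y axes.
; Completing the place action calls PlaceTrap and the close-edit action calls ToPlayer, neither of which is implemented in this graph.
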(event Input|EnhancedActionEvents|EnhancedInputActionCloseEditAction
  (params (ActionValue :type Boolean) (ElapsedSeconds :type Float%20%28double-precision%29) (TriggeredSeconds :type Float%20%28double-precision%29) (InputAction :type Input%20Action%20Object%20Reference :default "/Game/Blueprints/Demon/Inputs/CloseEditAction.CloseEditAction"))
  ;[1 0.1962 0.4495] To Player
  (:Triggered
    (Class|TrapPlacer|ToPlayer)))

(event Input|EnhancedActionEvents|EnhancedInputActionCursMoveAction
  (params (ActionValue :type Vector%202D%20Structure) (ElapsedSeconds :type Float%20%28double-precision%29) (TriggeredSeconds :type Float%20%28double-precision%29) (InputAction :type Input%20Action%20Object%20Reference :default "/Game/Blueprints/Demon/Inputs/CursMoveAction.CursMoveAction"))
  ;[0.3512 1 0.4852] Move Input
  (:Triggered
    (Pawn|Input|AddMovementInput "1.000000,0.000000,0.000000" (.y ActionValue) false)
    (Pawn|Input|AddMovementInput "0.000000,1.000000,0.000000" (.x ActionValue) false)))

(event Input|EnhancedActionEvents|EnhancedInputActionPlaceAction
  (params (ActionValue :type Boolean) (ElapsedSeconds :type Float%20%28double-precision%29) (TriggeredSeconds :type Float%20%28double-precision%29) (InputAction :type Input%20Action%20Object%20Reference :default "/Game/Blueprints/Demon/Inputs/PlaceAction.PlaceAction"))
  ;[1 0.6203 0.1906] Place Trap
  (:Completed
    (Class|TrapPlacer|PlaceTrap)))

(event EventBeginPlay
  (bind _asplayer_controller (Utilities|Casting|CastToPlayerController (Pawn|GetController)))
  (Utilities|IsValid (PlayerController|LocalPlayerSubsystems|GetEnhancedInputLocalPlayerSubsystem _asplayer_controller)
    (:Is%20Valid
      (Input|AddMappingContext (PlayerController|LocalPlayerSubsystems|GetEnhancedInputLocalPlayerSubsystem _asplayer_controller) "/Game/Blueprints/Demon/Inputs/InpuMapping.InpuMapping" 0 "(bIgnoreAllPressedKeysUntilRelease=True,bForceImmediately=False)"))))

(fn ConstructionScript)