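; Dungeon room actor that randomly picks a Basic or Bone type and dresses its placeholder meshes on BeginPlay.
; It scans all level StaticMeshActors for temp floor and wall meshes, swapping each by weighted rolls and randomly rotating floors.
; Failed rolls fall back to the highest floor-weight index, even for walls.
; It then updates BP_DungeonManager's waypoint list and next room position from RoomExit, then calls SetMissingWaypoints.
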(event Custom|DecorateRoom
  (CallFunction|GetFloors)
  (CallFunction|GetWallls)
  (CallFunction|ChangeFLoors)
  (CallFunction|ChangeWalls))

(event Custom|GetFloors
  ;[1 1 1] Get all floors
  (bind _outactors (Actor|GetAllActorsOfClass "/Script/Engine.StaticMeshActor"))
  (for _array_element _outactors
    (if (== (Variables|/Script/Engine.StaticMeshComponent|GetStaticMesh (Variables|/Script/Engine.StaticMeshActor|GetStaticMeshComponent _array_element)) "/Game/External_Assets/KayLousberg/DungeonPack/floor_tile_small_gltf_TEMP.floor_tile_small_gltf_TEMP")
      (Utilities|Array|Add (Variables|Default|GetTempFloorList) _array_element))))

(event Custom|ChangeWalls
  (CallFunction|ChangeRoomMeshes (Variables|Default|GetTempWallList) (Variables|Default|GetWallTypesRNG) (Variables|Default|GetWallTypes) false))

(event Custom|GetWallls
  ;[1 1 1] Get all walls
  (bind _outactors (Actor|GetAllActorsOfClass "/Script/Engine.StaticMeshActor"))
  (for _array_element _outactors
    (if (== (Variables|/Script/Engine.StaticMeshComponent|GetStaticMesh (Variables|/Script/Engine.StaticMeshActor|GetStaticMeshComponent _array_element)) "/Game/External_Assets/KayLousberg/DungeonPack/wall_gltf_TEMP.wall_gltf_TEMP")
      (Utilities|Array|Add (Variables|Default|GetTempWallList) _array_element))))

(event Custom|OnItemFound
  ;[1 1 1] Change Mesh Actor
  (Utilities|Array|ForEachLoopwithBreak (stale Custom|ChangeRoomMeshes MeshListRNG)) ; enters at Break
)

(event Custom|ChangeFloors
  (CallFunction|ChangeRoomMeshes (Variables|Default|GetTempFloorList) (Variables|Default|GetFloorTypesRNG) (Variables|Default|GetFloorTypes) true))

(event Custom|ChangeRoomMeshes
  (params (TempMeshList :type Array%20of%20Static%20Mesh%20Actor%20Object%20References) (MeshListRNG :type Array%20of%20Floats%20%28double-precision%29) (NewMeshList :type Array%20of%20Static%20Mesh%20Object%20References) (ChangeRot :type Boolean))
  ;[1 1 1] Change Mesh Actor
  (for _array_element TempMeshList
    (Variables|Default|SetItemFound false)
    (bind (_array_element_2 _array_index) (Utilities|Array|ForEachLoopwithBreak MeshListRNG)
      (:LoopBody
        (if (Math|Random|RandomBoolwithWeight _array_element_2)
          (CallFunction|OnItemFound)
          (Variables|Default|SetItemFound true)
          (Variables|Default|SetItemIndex _array_index)))
      (:Completed
        (if (Variables|Default|GetItemFound)
          _
          (else
            (bind _output_get (Variables|Default|SetItemIndex (.IndexOfMaxValue (Math|Float|MaxOfFloatArray (Variables|Default|GetFloorTypesRNG)))))))
        (Components|StaticMesh|SetStaticMesh (Variables|/Script/Engine.StaticMeshActor|GetStaticMeshComponent _array_element) (Utilities|Array|Get(acopy) NewMeshList _output_get))
        (if ChangeRot
          (switch int (Math|Random|RandomInteger 4)
            (:0
              (Transformation|SetActorRotation _array_element "0.000000,90.000000,0.000000"))
            (:1
              (Transformation|SetActorRotation _array_element "0.000000,180.000000,0.000000"))
            (:2
              (Transformation|SetActorRotation _array_element "0.000000,270.000000,0.000000"))))))))

(event EventBeginPlay
  ;[1 1 1] Set the room type
  (if (Math|Random|RandomBoolwithWeight 0.5)
    (Variables|Default|SetRoomType "Basic")
    (else
      (Variables|Default|SetRoomType "Bone")))
  (CallFunction|DecorateRoom)
  ;[1 1 1] Add Waypoints
  (bind _returnvalue (Actor|GetActorOfClass "/Game/Blueprints/Dungeon/BP_DungeonManager.BP_DungeonManager_C"))
  (bind _output_get (Variables|Default|SetAs_BP_DungeonManager _returnvalue))
  (for _array_element (Variables|/Script/ThisIsMyDungeon.DungeonManager|GetwaypointList _output_get)
    (Utilities|Array|Add (Variables|/Script/ThisIsMyDungeon.DungeonManager|GetWaypointList (Variables|Default|GetAs_BP_DungeonManager)) _array_element))
  (Variables|/Script/ThisIsMyDungeon.DungeonManager|SetNextRoomPos (Variables|Default|GetAs_BP_DungeonManager) (+ (- (Variables|Default|GetRoomExit) "0.000000,100.000000,0.000000") (Transformation|GetActorLocation)))
  (Class|DungeonManager|SetMissingWaypoints (Variables|Default|GetAs_BP_DungeonManager)))

(fn ConstructionScript)