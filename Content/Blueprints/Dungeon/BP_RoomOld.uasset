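; BP_RoomOld is a dungeon room that registers itself with the level's BP_DungeonManager on BeginPlay.
; It appends its RoomWaypoints to the manager's WaypointList and sets NextRoomPos to its RoomExit offset plus its actor location, ignoring rotation.
; It then calls SetMissingWaypoints on the manager; the construction script is empty.
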(event EventBeginPlay
  (bind _returnvalue (Actor|GetActorOfClass "/Game/Blueprints/Dungeon/BP_DungeonManager.BP_DungeonManager_C"))
  (Variables|Default|SetAs_BP_DungeonManager _returnvalue)
  (for _array_element (Variables|Default|GetRoomWaypoints)
    (Utilities|Array|Add (Variables|/Script/ThisIsMyDungeon.DungeonManager|GetWaypointList (Variables|Default|GetAs_BP_DungeonManager)) _array_element))
  (Variables|/Script/ThisIsMyDungeon.DungeonManager|SetNextRoomPos (Variables|Default|GetAs_BP_DungeonManager) (+ (Variables|Default|GetRoomExit) (Transformation|GetActorLocation)))
  (Class|DungeonManager|SetMissingWaypoints (Variables|Default|GetAs_BP_DungeonManager)))

(fn ConstructionScript)