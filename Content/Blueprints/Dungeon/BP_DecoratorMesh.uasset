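; BP_DecoratorMesh is a dungeon decorator that randomly scatters static mesh decorations within its box bounds on BeginPlay.
; Each spawn attempt passes a weighted chance, then spawns a BP_Decoration at a random XY in the box, at the actor's height with random yaw.
; Each decoration gets a randomly picked mesh from ActorsToSpawn.
; DoCollision only toggles overlap events on the bounds box, while spawn collision handling is left undefined.
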(event EventBeginPlay
  (bind _boxbounds (Variables|Default|GetBoxBounds))
  (bind _defaultsceneroot (Variables|Default|GetDefaultSceneRoot))
  (bind _boxbounds_2 (Variables|Default|GetBoxBounds))
  (bind _returnvalue (Transformation|GetWorldLocation _defaultsceneroot))
  (bind _returnvalue_2 (Components|Box|GetScaledBoxExtent _boxbounds_2))
  (bind _returnvalue_3 (Math|Random|RandomPointinBoundingBox _returnvalue _returnvalue_2))
  (bind _returnvalue_4 (Math|Conversions|ToTransform(Vector) _returnvalue_3))
  (if (Variables|Default|GetDoCollision)
    (Variables|/Script/Engine.PrimitiveComponent|SetbGenerateOverlapEvents _boxbounds true)
    (else
      (Variables|/Script/Engine.PrimitiveComponent|SetbGenerateOverlapEvents _boxbounds false)))
  (for _index (range 0 (- (Variables|Default|GetAmountToSpawn) 1))
    (if (Math|Random|RandomBoolwithWeight (Variables|Default|GetSpawnRNG))
      (Variables|Default|SetMeshRNG (Math|Random|RandomInteger (Utilities|Array|Length (Variables|Default|GetActorsToSpawn))))
      (for (_array_element _array_index) (Variables|Default|GetActorsToSpawn)
        (if (== _array_index (Variables|Default|GetMeshRNG))
          (bind _returnvalue_5 (Game|SpawnActorfromClass "/Game/Blueprints/Dungeon/BP_Decoration.BP_Decoration_C" (Math|Transform|MakeTransform (Math|Vector|MakeVector (.x (.location _returnvalue_4)) (.y (.location _returnvalue_4)) (.z (Transformation|GetActorLocation))) (Math|Rotator|MakeRotator 0.0 0.0 (Math|Random|RandomFloatinRange 0.0 3.6e+02)) (.scale _returnvalue_4)) "Undefined" "MultiplyWithRoot" 0 0))
          (Components|StaticMesh|SetStaticMesh (Variables|/Game/Blueprints/Dungeon/BP_Decoration.BP_Decoration_C|GetStaticMesh _returnvalue_5) _array_element))))))

(fn ConstructionScript)