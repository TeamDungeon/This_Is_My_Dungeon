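; Dungeon manager that grows the dungeon by streaming in room levels as hero waves progress.
; BeginPlay loads the treasure room, then after a short delay caches the HeroSpawner and enables spawning.
; Tick watches the spawner's CurrentWave and fires a DoOnce per wave for the first eight waves to add a room.
; Each addition updates RoomList and loads the next room as a level instance at its position, capped by a temporary counter.
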(event Custom|GenerateNewRoom
  ;[1 1 1] Generate Room
  (if (Utilities|Array|IsNotEmpty (Variables|Default|GetRoomList))
    (Class|DungeonManager|UpdateRoomList)
    (Class|LevelStreamingDynamic|LoadLevelInstance (Variables|Default|GetNextRoomName) (Variables|Default|GetNextRoomPos) "0, 0, 0" "" 0 false)))

(event Custom|TEMP_AddRoom
  ;[1 1 1] Loop to add several rooms
  (if (<= (Variables|Default|GetTEMP_Tracker) (Variables|Default|GetTEMP_RoomListDefaultSize))
    (CallFunction|GenerateNewRoom)
    (Variables|Default|SetTEMP_Tracker (+ (Variables|Default|GetTEMP_Tracker) 1))
    (Utilities|FlowControl|Delay 1.0)))

(event EventBeginPlay
  ;[1 1 1] Begin
  (Variables|Default|SetTEMP_Tracker 0)
  (Variables|Default|SetTEMP_RoomListDefaultSize (Utilities|Array|Length (Variables|Default|GetRoomList)))
  (Variables|Default|SetIsTreasureRoom true)
  (Class|LevelStreamingDynamic|LoadLevelInstance "TreasureRoom" "0, 0, 0" "0, 0, 0" "" 0 false)
  (Utilities|FlowControl|Delay 1.0)
  (bind _returnvalue (Actor|GetActorOfClass "/Script/ThisIsMyDungeon.HeroSpawner"))
  (Variables|Default|SetAs%20Hero%20Spawner _returnvalue)
  (Variables|Default|SetCanSpawn true))

(event EventTick
  (params (DeltaSeconds :type Float%20%28single-precision%29))
  (if (Variables|Default|GetCanSpawn)
    (switch int (Variables|/Script/ThisIsMyDungeon.HeroSpawner|GetcurrentWave (Variables|Default|GetAs%20Hero%20Spawner))
      (:0
        (Utilities|FlowControl|DoOnce false
          (:Completed
            (CallFunction|TEMPAddRoom))))
      (:1
        (Utilities|FlowControl|DoOnce false
          (:Completed
            (CallFunction|TEMPAddRoom))))
      (:2
        (Utilities|FlowControl|DoOnce false
          (:Completed
            (CallFunction|TEMPAddRoom))))
      (:3
        (Utilities|FlowControl|DoOnce false
          (:Completed
            (CallFunction|TEMPAddRoom))))
      (:4
        (Utilities|FlowControl|DoOnce false
          (:Completed
            (CallFunction|TEMPAddRoom))))
      (:5
        (Utilities|FlowControl|DoOnce false
          (:Completed
            (CallFunction|TEMPAddRoom))))
      (:6
        (Utilities|FlowControl|DoOnce false
          (:Completed
            (CallFunction|TEMPAddRoom))))
      (:7
        (Utilities|FlowControl|DoOnce false
          (:Completed
            (CallFunction|TEMPAddRoom)))))))

(fn ConstructionScript)