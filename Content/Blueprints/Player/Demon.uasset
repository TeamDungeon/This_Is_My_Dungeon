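; Demon is the player character Blueprint, handling camera look, movement, fireball shooting and an editor action through Enhanced Input.
; BeginPlay registers the input mapping context and adds coin and mana counter widgets to the viewport.
; Movement follows control yaw, turning off orient-to-movement while input is held and lerping actor yaw toward the camera by elapsed input time.
; Shoot calls SpawnFireball on completion, and the editor action calls ToEdit.
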(event Input|EnhancedActionEvents|EnhancedInputActionLookAction
  (params (ActionValue :type Vector%202D%20Structure) (ElapsedSeconds :type Float%20%28double-precision%29) (TriggeredSeconds :type Float%20%28double-precision%29) (InputAction :type Input%20Action%20Object%20Reference :default "/Game/Blueprints/Player/Inputs/LookAction.LookAction"))
  ;[0.1768 1 0.4743] Camera
  (:Triggered
    (Pawn|Input|AddControllerYawInput (* (.x ActionValue) -1.0))
    (Pawn|Input|AddControllerPitchInput (.y ActionValue))))

(event Input|EnhancedActionEvents|EnhancedInputActionMoveAction
  (params (ActionValue :type Vector%202D%20Structure) (ElapsedSeconds :type Float%20%28double-precision%29) (TriggeredSeconds :type Float%20%28double-precision%29) (InputAction :type Input%20Action%20Object%20Reference :default "/Game/Blueprints/Player/Inputs/MoveAction.MoveAction"))
  (bind _returnvalue (Pawn|GetControlRotation :!class /Script/Engine.Pawn))
  (bind _charactermovement (Variables|Character|GetCharacterMovement))
  ;[0.3229 0.7447 1] Movement
  (:Triggered
    ;;[1 1 1] smooth  Rotation of the player
    (Transformation|SetActorRotation (Math|Rotator|MakeRotator 0.0 0.0 (Math|Float|Lerp (.yaw (Transformation|GetActorRotation)) (.yaw (Transformation|GetWorldRotation (Variables|Default|GetCamera1))) (Math|Float|Clamp(Float) ElapsedSeconds))))
    (Pawn|Input|AddMovementInput (Math|Vector|GetRightVector (Math|Rotator|MakeRotator (.roll _returnvalue) 0.0 (.yaw _returnvalue))) (.x ActionValue) false)
    (Pawn|Input|AddMovementInput (Math|Vector|GetForwardVector (Math|Rotator|MakeRotator 0.0 0.0 (.yaw (Pawn|GetControlRotation :!class /Script/Engine.Pawn)))) (.y ActionValue) false))
  (:Started
    ;;[1 1 1] On start set action to False on end set to True
    (Variables|/Script/Engine.CharacterMovementComponent|SetbOrientRotationToMovement _charactermovement false))
  (:Completed
    (Variables|/Script/Engine.CharacterMovementComponent|SetbOrientRotationToMovement _charactermovement true)))

(event Input|EnhancedActionEvents|EnhancedInputActionToEditorAction
  (params (ActionValue :type Boolean) (ElapsedSeconds :type Float%20%28double-precision%29) (TriggeredSeconds :type Float%20%28double-precision%29) (InputAction :type Input%20Action%20Object%20Reference :default "/Game/Blueprints/Player/Inputs/ToEditorAction.ToEditorAction"))
  ;[1 1 1] ToEditor
  (:Triggered
    (Class|Demon|ToEdit)))

(event Input|EnhancedActionEvents|EnhancedInputActionShootAction
  (params (ActionValue :type Boolean) (ElapsedSeconds :type Float%20%28double-precision%29) (TriggeredSeconds :type Float%20%28double-precision%29) (InputAction :type Input%20Action%20Object%20Reference :default "/Game/Blueprints/Player/Inputs/ShootAction.ShootAction"))
  ;[1 1 1] Shoot
  (:Completed
    (Class|Demon|SpawnFireball)))

(event EventBeginPlay
  ;[0.7614 1 0.303] Add_Controller
  (bind _asplayer_controller (Utilities|Casting|CastToPlayerController (Pawn|GetController)))
  (Utilities|IsValid (PlayerController|LocalPlayerSubsystems|GetEnhancedInputLocalPlayerSubsystem _asplayer_controller)
    (:Is%20Valid
      (Input|AddMappingContext (PlayerController|LocalPlayerSubsystems|GetEnhancedInputLocalPlayerSubsystem _asplayer_controller) "/Game/Blueprints/Player/Inputs/InpuMapping.InpuMapping" 0 "(bIgnoreAllPressedKeysUntilRelease=True,bForceImmediately=False)")
      ;[1 0.4586 0.7295] UI
      (bind _returnvalue (UserInterface|CreateWidget "/Game/Blueprints/Player/UI/CoinCounterWidget.CoinCounterWidget_C"))
      (bind _returnvalue_2 (UserInterface|CreateWidget "/Game/Blueprints/Player/UI/ManaCounterWidget.ManaCounterWidget_C"))
      (UserInterface|Viewport|AddtoViewport _returnvalue 0))))

(fn ConstructionScript)